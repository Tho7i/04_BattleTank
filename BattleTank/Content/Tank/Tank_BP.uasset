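; Player-controlled tank Blueprint that handles firing and orbiting the aim camera.
; On BeginPlay it registers its turret and barrel components through SetTurretReference and SetBarrelReference, and the Fire input calls Fire, none of which are defined in this graph.
; Azimuth input yaws the AzimuthGimbal and elevation input pitches the SpringArm separately, both scaled by delta time for frame-rate-independent rotation.
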(event EventBeginPlay
  (Class|Tank|SetTurretReference (Variables|Default|GetTankTurret))
  (Class|Tank|SetBarrelReference (Variables|Default|GetTankBarrel)))

(event Input|ActionEvents|InputActionFire
  (params (Key :type Key%20Structure :default "None"))
  (:Pressed
    (Class|Tank|Fire)))

(event Input|AxisEvents|InputAxisAimAzimuth
  (params (AxisValue :type Float%20%28single-precision%29))
  ;[1 1 1] Camera Rotation
  (Transformation|AddLocalRotation (Variables|Default|GetAzimuth%20Gimbal) (Math|Rotator|MakeRotator 0.0 0.0 (* AxisValue (Utilities|Time|GetWorldDeltaSeconds) 1e+02)) false false))

(event Input|AxisEvents|InputAxisAimElevation
  (params (AxisValue :type Float%20%28single-precision%29))
  ;[1 1 1] Camera Rotation
  (Transformation|AddLocalRotation (Variables|Default|GetSpring%20Arm) (Math|Rotator|MakeRotator 0.0 (* AxisValue (Utilities|Time|GetWorldDeltaSeconds) 1e+02) 0.0) false false))

(fn ConstructionScript)